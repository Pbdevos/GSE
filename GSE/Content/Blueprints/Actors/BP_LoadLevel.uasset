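; Level transition trigger actor that streams in the next level or ends the demo when the third-person character overlaps it.
; Normally it loads LevelToLoad as visible without blocking and teleports the character to the PlayerLocation component.
; With EndDemo set, it skips loading, shows the main menu and cursor, moves the character to the PlayerStart and unloads CurrentLevel.
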(event `self.ReceiveBeginPlay`
  (set `PlayerController.bShowMouseCursor` false (`GameplayStatics.GetPlayerController` 0)))

(event `self.ReceiveActorBeginOverlap`
  (params (OtherActor :type "Actor Object Reference"))
  (bind _asbp_third_person_character (cast `/Game/ThirdPerson/Blueprints/BP_ThirdPersonCharacter` OtherActor))
  (if (not (`self.EndDemo`))
    (`GameplayStatics.LoadStreamLevelBySoftObjectPtr` (`self.LevelToLoad`) true))
  (`self.K2_SetActorLocation` _asbp_third_person_character (`SceneComponent.K2_GetComponentLocation` (`self.PlayerLocation`)) false true)
  (if (`self.EndDemo`)
    (bind _returnvalue (`|CreateWidget` "/Game/Blueprints/Widgets/WBP_MainMenu.WBP_MainMenu_C"))
    (`UserWidget.AddToViewport` _returnvalue 0)
    (set `PlayerController.bShowMouseCursor` true (`GameplayStatics.GetPlayerController` 0))
    (bind _returnvalue_2 (`GameplayStatics.GetActorOfClass` "/Game/ThirdPerson/Blueprints/BP_ThirdPersonCharacter.BP_ThirdPersonCharacter_C"))
    (bind _returnvalue_3 (`GameplayStatics.GetActorOfClass` "/Script/Engine.PlayerStart"))
    (`self.K2_SetActorLocation` _returnvalue_2 (`self.K2_GetActorLocation` _returnvalue_3) false false)
    (`GameplayStatics.UnloadStreamLevelBySoftObjectPtr` (`self.CurrentLevel`))))

(fn `UserConstructionScript`)