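; BP_GSEGameInstance is a game instance that owns background music and starts a Twinsen's Little Big Adventure remix track on Init, along with a debug "Hello" print.
; PlayMusic fades out the current audio component, spawns the new track as a 2D sound, fades it in and stores it as CurrentMusic.
; The same-track comparison and Stop nodes are unconnected, so replaying the current track restarts it.
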(event `self.ReceiveInit`
  (`self.PlayMusic` "/Game/Audio/Music/Little_Big_Adventure_Remix___Twinsen_of_Twinsun_-zxUDtQxNPTs_1.Little_Big_Adventure_Remix___Twinsen_of_Twinsun_-zxUDtQxNPTs_1")
  (`KismetSystemLibrary.PrintString` "Hello"))

(fn `PlayMusic`
  (params (NewMusic :type "SoundBase Object Reference"))
  (bind _musiccomponent (`self.MusicComponent`))
  (set `self.New Music` NewMusic)
  (`/Engine/EditorBlueprintResources/StandardMacros.IsValid` (`self.New Music`)
    (:`Is Valid`
      (`/Engine/EditorBlueprintResources/StandardMacros.IsValid` _musiccomponent
        (:`Is Valid`
          (`AudioComponent.FadeOut` _musiccomponent 1.0 0.0 "Linear"))
        (:`Is Not Valid`
          _))
      (bind _returnvalue (`GameplayStatics.SpawnSound2D` (`self.New Music`) 1.0 1.0 0.0 null))
      (bind _output_get (set `self.MusicComponent` _returnvalue))
      (`AudioComponent.FadeIn` _output_get 1.0 1.0 0.0 "Linear")
      (set `self.CurrentMusic` (`self.New Music`)))))